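; BP_Switch is a light switch that toggles a point light, a spark and an electric hum when E is pressed.
; A trigger enables input only while the third-person character overlaps it, and a FlipFlop alternates visibility and hum activation.
; Everything starts off on BeginPlay.
; A separate Interact event flips IsLightOn and prints the state without affecting these components or the FlipFlop.
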(event `/Game/LightSwitch/BPI_Interact.Interact`
  (if (not (`self.IsLightOn`))
    (set `self.IsLightOn` true)
    (`KismetSystemLibrary.PrintString` "Light On")
    (else
      (set `self.IsLightOn` false)
      (`KismetSystemLibrary.PrintString` "Light Off"))))

(event `self.Trigger.OnComponentBeginOverlap`
  (params (OverlappedComponent :type "PrimitiveComponent Object Reference") (OtherActor :type "Actor Object Reference") (OtherComp :type "PrimitiveComponent Object Reference") (OtherBodyIndex :type Integer) (bFromSweep :type Boolean) (SweepResult :type "HitResult Structure (by ref)"))
  (cast `/Game/ThirdPerson/Blueprints/BP_ThirdPersonCharacter` OtherActor)
  (`self.EnableInput` (`GameplayStatics.GetPlayerController` 0)))

(event `self.Trigger.OnComponentEndOverlap`
  (params (OverlappedComponent :type "PrimitiveComponent Object Reference") (OtherActor :type "Actor Object Reference") (OtherComp :type "PrimitiveComponent Object Reference") (OtherBodyIndex :type Integer))
  (cast `/Game/ThirdPerson/Blueprints/BP_ThirdPersonCharacter` OtherActor)
  (`self.DisableInput` (`GameplayStatics.GetPlayerController` 0)))

(event `Key|E`
  (params (Key :type "Key Structure"))
  (bind _pointlight (`self.PointLight`))
  (bind _electric_hum_141075 (`self.electric-hum-141075`))
  (:`Pressed`
    (`/Engine/EditorBlueprintResources/StandardMacros.FlipFlop`
      (:`A`
        (`SceneComponent.SetVisibility` _pointlight true false)
        (`SceneComponent.SetVisibility` (`self.spark`) true false)
        (`ActorComponent.SetActive` _electric_hum_141075 true false))
      (:`B`
        (`SceneComponent.SetVisibility` _pointlight false false)
        (`SceneComponent.SetVisibility` (`self.spark`) false false)
        (`ActorComponent.SetActive` _electric_hum_141075 false false)))))

(event `self.ReceiveBeginPlay`
  (`SceneComponent.SetVisibility` (`self.PointLight`) false false)
  (`SceneComponent.SetVisibility` (`self.spark`) false false)
  (`ActorComponent.SetActive` (`self.electric-hum-141075`) false false))

(fn `UserConstructionScript`)