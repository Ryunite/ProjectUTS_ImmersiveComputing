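; Horror light switch actor that toggles a spotlight and plane in opposition, with a death trigger.
; Overlapping SwitchTrigger enables player input so E flip-flops their visibility; the first press repeats the BeginPlay state of light visible, plane hidden.
; A separate Interact event only toggles IsLightOn and prints it.
; DeathTriggerBox activates the jumpscare component and sets the character mesh simulating physics.
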(event `self.Interact`
  (if (not (`self.IsLightOn`))
    (set `self.IsLightOn` true)
    (`KismetSystemLibrary.PrintString` "Light On")
    (else
      (set `self.IsLightOn` false)
      (`KismetSystemLibrary.PrintString` "Light Off"))))

(event `self.SwitchTrigger.OnComponentBeginOverlap`
  (params (OverlappedComponent :type "PrimitiveComponent Object Reference") (OtherActor :type "Actor Object Reference") (OtherComp :type "PrimitiveComponent Object Reference") (OtherBodyIndex :type Integer) (bFromSweep :type Boolean) (SweepResult :type "HitResult Structure (by ref)"))
  (cast `/Game/ThirdPerson/Blueprints/BP_ThirdPersonCharacter` OtherActor)
  (`self.EnableInput` (`GameplayStatics.GetPlayerController` 0)))

(event `self.SwitchTrigger.OnComponentEndOverlap`
  (params (OverlappedComponent :type "PrimitiveComponent Object Reference") (OtherActor :type "Actor Object Reference") (OtherComp :type "PrimitiveComponent Object Reference") (OtherBodyIndex :type Integer))
  (cast `/Game/ThirdPerson/Blueprints/BP_ThirdPersonCharacter` OtherActor)
  (`self.DisableInput` (`GameplayStatics.GetPlayerController` 0)))

(event `Key|E`
  (params (Key :type "Key Structure"))
  (bind _spotlight (`self.SpotLight`))
  (bind _plane (`self.Plane`))
  (:`Pressed`
    (`/Engine/EditorBlueprintResources/StandardMacros.FlipFlop`
      (:`A`
        (`SceneComponent.SetVisibility` _spotlight true false)
        (`SceneComponent.SetVisibility` _plane false false))
      (:`B`
        (`SceneComponent.SetVisibility` _spotlight false false)
        (`SceneComponent.SetVisibility` _plane true false)))))

(event `self.ReceiveBeginPlay`
  (`SceneComponent.SetVisibility` (`self.SpotLight`) true false)
  (`SceneComponent.SetVisibility` (`self.Plane`) false false))

(event `self.DeathTriggerBox.OnComponentBeginOverlap`
  (params (OverlappedComponent :type "PrimitiveComponent Object Reference") (OtherActor :type "Actor Object Reference") (OtherComp :type "PrimitiveComponent Object Reference") (OtherBodyIndex :type Integer) (bFromSweep :type Boolean) (SweepResult :type "HitResult Structure (by ref)"))
  (bind _asbp_third_person_character (cast `/Game/ThirdPerson/Blueprints/BP_ThirdPersonCharacter` OtherActor))
  (`ActorComponent.Activate` (`self.jumpscare-94984`) false)
  (`PrimitiveComponent.SetSimulatePhysics` (`Character.Mesh` _asbp_third_person_character) true))

(fn `UserConstructionScript`)